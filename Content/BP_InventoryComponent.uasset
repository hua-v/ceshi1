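; Inventory component that holds an Items array and a selected slot index, with slot cycling, lookup and drop functions.
; NextSlot and PrevSlot wrap the index by MaxSlots and pass it to SelectSlot, whose bounds-check and update logic is unconnected, so selection never changes.
; GetSelectedItem reads the slot after a validity check.
; DropSelected removes and returns the item unchecked, then fires OnSelectionChanged.
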(fn `DropSelected`
  (returns (NewParam :type "/Game/F_ItemData Structure"))
  (locals (Dropped :type "/Game/F_ItemData Structure"))
  (bind _selectedindex (`self.SelectedIndex`))
  (set `local.Dropped` (`|GetArrayItem` (`self.Items`) _selectedindex))
  (`KismetArrayLibrary.Array_Remove` (`self.Items`) _selectedindex)
  (`self.OnSelectionChanged` _selectedindex)
  (return (`local.Dropped`)))

(fn `Get Selected Item`
  (returns (NewParam :type "/Game/F_ItemData Structure") (Result1 :type "/Game/F_ItemData Structure") (Result2 :type "/Game/F_ItemData Structure") (Result3 :type "/Game/F_ItemData Structure"))
  (locals (Result :type "/Game/F_ItemData Structure"))
  (bind _selectedindex (`self.SelectedIndex`))
  (bind _result (`local.Result`))
  (if (`KismetArrayLibrary.Array_IsValidIndex` (`self.Items`) _selectedindex)
    (set `local.Result` (`|GetArrayItem` (`self.Items`) _selectedindex)))
  (return _result _result _result _result))

(fn `NextSlot`
  (`self.Select Slot` (mod (+ (`self.SelectedIndex`) 1) (`self.MaxSlots`))))

(fn `Prev Slot`
  (`self.Select Slot` (mod (+ (- (`self.SelectedIndex`) 1) (`self.MaxSlots`)) (`self.MaxSlots`))))

(fn `Select Slot`
  (params (NewIndex :type Integer)))